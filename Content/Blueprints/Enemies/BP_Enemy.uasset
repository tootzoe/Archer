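; BP_Enemy is an enemy Blueprint that handles basic visual setup and death feedback.
; On BeginPlay it binds to the character-dead event, whose handler switches the static mesh's first material slot to M_Base.
; If the skeletal Mesh has an asset, BeginPlay also deactivates the StaticMesh component and calls SetAnimInstanceClass with no class specified.
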(event Custom|OnCharacterDead_Event_0
  (Rendering|Material|SetMaterial (Variables|Default|GetStaticMesh) 0 "/Game/Materials/M_Base.M_Base"))

(event EventBeginPlay
  (EventDispatchers|AssignOnCharacterDead (delegate Custom|OnCharacterDead_Event_0))
  (Utilities|IsValid (Class|SkinnedMeshComponent|GetSkinnedAsset (Variables|Character|GetMesh))
    (:Is%20Valid
      (Components|Activation|Deactivate (Variables|Default|GetStaticMesh))
      (Components|SkeletalMesh|SetAnimInstanceClass (Variables|Character|GetMesh) 0))))

(event Collision|EventActorBeginOverlap
  (params (OtherActor :type Actor%20Object%20Reference)))

(event EventTick
  (params (DeltaSeconds :type Float%20%28single-precision%29)))

(fn ConstructionScript)