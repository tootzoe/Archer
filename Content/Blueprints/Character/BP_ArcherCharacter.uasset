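; BP_ArcherCharacter is an archer character Blueprint that chooses between a skeletal and a static mesh for its visual representation.
; On BeginPlay it checks whether the skeletal Mesh has a valid asset and, if so, deactivates and hides the StaticMesh.
; Otherwise it clears the anim instance class and deactivates and hides the skeletal Mesh, leaving the StaticMesh as the fallback visual.
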(event EventBeginPlay
  (bind _mesh (Variables|Character|GetMesh))
  (bind _staticmesh (Variables|Default|GetStaticMesh))
  (Utilities|IsValid (Class|SkinnedMeshComponent|GetSkinnedAsset (Variables|Character|GetMesh))
    (:Is%20Valid
      (Components|Activation|Deactivate _staticmesh)
      (Rendering|SetVisibility _staticmesh false false))
    (:Is%20Not%20Valid
      (Components|SkeletalMesh|SetAnimInstanceClass (Variables|Character|GetMesh) 0)
      (Components|Activation|Deactivate _mesh)
      (Rendering|SetVisibility _mesh false false))))

(fn ConstructionScript)